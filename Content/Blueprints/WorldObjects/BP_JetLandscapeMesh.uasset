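; BP_JetLandscapeMesh is a procedural-mesh landscape actor for the Jet game, sized by tile size and landscape size.
; SmoothDestroy turns off mesh collision and sets the life span to zero, which clears any expiry timer rather than destroying the actor.
; GetCenterLocation offsets the actor location by half the landscape extent in X and Y.
; BeginPlay and Tick only call the parent; player-exit and self-destroy logic is disconnected.
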(event `self.ReceiveBeginPlay`
  (`parent.ReceiveBeginPlay`))

(event `self.ReceiveTick`
  (params (DeltaSeconds :type "Float (single-precision)"))
  (`parent.ReceiveTick` DeltaSeconds))

(event `self.SmoothDestroy`
  (`PrimitiveComponent.SetCollisionEnabled` (`self.ProcMesh`) "NoCollision")
  (`self.SetLifeSpan` 0.0))

(fn `GetCenterLocation`
  (returns (ReturnValue :type "Vector Structure"))
  (bind _returnvalue (`KismetMathLibrary.Conv_IntToDouble` (/ (* (`self.TileSize`) (`self.LandscapeSize`)) 2)))
  (return (+ (`self.K2_GetActorLocation`) (`KismetMathLibrary.MakeVector` _returnvalue _returnvalue))))

(fn `UserConstructionScript`)