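; World spawner Blueprint that drives periodic landscape updates and places the jet character on the ground once the world spawns.
; A looping timer from BeginPlay calls UpdateLandscape and prints a debug message.
; On the first OnWorldSpawned, another timer repeats a vertical object trace around the player until it hits, then snaps the capsule onto the surface and sets gravity scale to normal.
; Level-streaming nodes are left unconnected.
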(event `self.ReceiveBeginPlay`
  (`parent.ReceiveBeginPlay`)
  (bind _returnvalue (`KismetSystemLibrary.K2_SetTimerDelegate` (delegate `CustomEvent_0`) 10.0 true))
  (set `self.UpdateLandscapeTimer` _returnvalue))

(event `CustomEvent_0`
  (`self.UpdateLandscape`)
  (`KismetSystemLibrary.PrintString` "UPDAATE" true true (struct :`G` 0.66 :`B` 1.0 :`A` 1.0) 5.0))

(event `self.ReceiveTick`
  (params (DeltaSeconds :type "Float (single-precision)"))
  (`parent.ReceiveTick` DeltaSeconds))

(event `OnLandscapesFinishedSpawning_1`
  (`|ExecutionSequence`))

(event `self.OnWorldSpawned`
  (if (not (`self.bHasWorldSpawned`))
    (set `self.bHasWorldSpawned` true)
    (cast `/Game/Blueprints/Character/BP_JetCharacter` (`GameplayStatics.GetPlayerCharacter` 0))
    (`|ExecutionSequence`
      (:`then_1`
        (if (not (`self.bGroundedPlayer`))
          (bind _returnvalue (`KismetSystemLibrary.K2_SetTimerDelegate` (delegate `GroundThePlayer`) 0.1 true))
          (set `self.GroundPlayerTimer` _returnvalue))))))

(event `GroundThePlayer`
  (bind _asbp_jet_character (cast `/Game/Blueprints/Character/BP_JetCharacter` (`GameplayStatics.GetPlayerCharacter` 0)))
  (bind _returnvalue (`self.K2_GetActorLocation` _asbp_jet_character))
  (bind (_outhit _returnvalue_2) (`KismetSystemLibrary.LineTraceSingleForObjects` :`Start` (+ _returnvalue (`KismetMathLibrary.MakeVector` 0.0 0.0 -5000.0)) :`End` (+ _returnvalue (`KismetMathLibrary.MakeVector` 0.0 0.0 5000.0)) :`ObjectTypes` (`|MakeArray` "ObjectTypeQuery7" :!type "EObjectTypeQuery Enum") :`bIgnoreSelf` false :`DrawTime` 20.0))
  (if _returnvalue_2
    (`self.K2_SetActorLocation` _asbp_jet_character (+ (`.ImpactPoint` (`GameplayStatics.BreakHitResult` _outhit)) (`KismetMathLibrary.MakeVector` 0.0 0.0 (`CapsuleComponent.GetScaledCapsuleHalfHeight` (`Character.CapsuleComponent` _asbp_jet_character)))) false false)
    (`KismetSystemLibrary.K2_ClearAndInvalidateTimerHandle` (`self.GroundPlayerTimer`))
    (set `self.bGroundedPlayer` true)
    (set `CharacterMovementComponent.GravityScale` 1.0 (`Character.CharacterMovement` _asbp_jet_character))))

(fn `UserConstructionScript`)