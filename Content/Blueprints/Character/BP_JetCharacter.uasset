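; Player character that tracks its position over the game's landscape tiles to notify them as it moves.
; Each Tick it finds the landscape under it by XY bounds in the GameState's SortedLandscapeArray, then derives a center-relative segment vector (signed step or zero per axis).
; A segment change prints debug text and calls that landscape's OnPlayerEnteredLandscape.
; A legacy check still updates current and previous landscape references, but its enter/exit calls are disconnected.
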(event `self.ReceiveBeginPlay`
  (`parent.ReceiveBeginPlay`))

(event `self.ReceiveTick`
  (params (DeltaSeconds :type "Float (single-precision)"))
  (`parent.ReceiveTick` DeltaSeconds)
  (`self.CheckLandscapeSpawn`)
  (`self.CheckLandscapeSpawnOld`))

(event `CheckLandscapeSpawnOld`
  (bind _outlandscape (`self.GetPlayerCurrentLandscape`))
  (`/Engine/EditorBlueprintResources/StandardMacros.IsValid` _outlandscape
    (:`Is Valid`
      (if (!= _outlandscape (`self.CurrentLandscape`))
        (`|ExecutionSequence`
          (:`then_0`
            (bind _currentlandscape (`self.CurrentLandscape`)
              (:`then`
                (set `self.PreviousLandscape` _currentlandscape))
              (:`else`)))
          (:`then_1`
            (bind _output_get (set `self.CurrentLandscape` _outlandscape))))))
    (:`Is Not Valid`
      (set `self.CurrentLandscape` null))))

(event `CheckLandscapeSpawn`
  (bind _outlandscape (`self.GetPlayerCurrentLandscape`))
  (bind _outlandscapesegmentvector (`self.GetPlayerCurrentLandscapeSegment`))
  (`/Engine/EditorBlueprintResources/StandardMacros.IsValid` _outlandscape
    (:`Is Valid`
      (if (!= _outlandscapesegmentvector (`self.LandscapeSegmentVector`))
        (set `self.LandscapeSegmentVector` _outlandscapesegmentvector)
        (`KismetSystemLibrary.PrintString` (`KismetStringLibrary.Conv_VectorToString` (`self.LandscapeSegmentVector`)) true true (struct :`G` 0.66 :`B` 1.0 :`A` 1.0) 20.0)
        (`JetLandscapeMesh.OnPlayerEnteredLandscape` _outlandscape self (`self.LandscapeSegmentVector`))))))

(fn `GetPlayerCurrentLandscape`
  (returns (OutLandscape :type "/Game/Blueprints/WorldObjects/BP_JetLandscapeMesh Object Reference"))
  (bind _asbp_jet_game_state (cast `/Game/Blueprints/GameState/BP_JetGameState` (`GameplayStatics.GetGameState`)))
  (for _array_element (`/Game/Blueprints/GameState/BP_JetGameState.SortedLandscapeArray` _asbp_jet_game_state)
    (bind _x (.x (`self.K2_GetActorLocation` _array_element)))
    (bind _y (.y (`self.K2_GetActorLocation` _array_element)))
    (bind _returnvalue (`JetLandscapeMesh.GetLandscapeScale` (`JetLandscapeMesh.LandscapeProperties` _array_element)))
    (if (and (`KismetMathLibrary.InRange_FloatFloat` (.x (`self.K2_GetActorLocation`)) _x (+ _x _returnvalue)) (`KismetMathLibrary.InRange_FloatFloat` (.y (`self.K2_GetActorLocation`)) _y (+ _y _returnvalue)))
      (return _array_element))))

(fn `GetPlayerCurrentLandscapeSegment`
  (returns (OutLandscapeSegmentVector :type "Vector Structure"))
  (bind _outlandscape (`self.GetPlayerCurrentLandscape`))
  (bind _landscapeproperties (`JetLandscapeMesh.LandscapeProperties` _outlandscape))
  (bind _returnvalue (`JetLandscapeMesh.GetLandscapeScale` _landscapeproperties))
  (bind _returnvalue_2 (/ _returnvalue 2.0))
  (bind _returnvalue_3 (`KismetMathLibrary.Abs` (/ _returnvalue (`.LandscapeSubdivisions` (break `LandscapeProperties` _landscapeproperties)))))
  (bind _x (.x (- (`self.K2_GetActorLocation`) (+ (`self.K2_GetActorLocation` _outlandscape) (`KismetMathLibrary.MakeVector` _returnvalue_2 _returnvalue_2)))))
  (bind _y (.y (- (`self.K2_GetActorLocation`) (+ (`self.K2_GetActorLocation` _outlandscape) (`KismetMathLibrary.MakeVector` _returnvalue_2 _returnvalue_2)))))
  (`/Engine/EditorBlueprintResources/StandardMacros.IsValid` _outlandscape
    (:`Is Valid`
      (return (`KismetMathLibrary.MakeVector` (* _returnvalue_3 (`KismetMathLibrary.SelectFloat` (`KismetMathLibrary.SignOfFloat` _x) 0.0 (> (`KismetMathLibrary.Abs` _x) _returnvalue_3))) (* _returnvalue_3 (`KismetMathLibrary.SelectFloat` (`KismetMathLibrary.SignOfFloat` _y) 0.0 (> (`KismetMathLibrary.Abs` _y) _returnvalue_3))))))))

(fn `IsPlayerWithinLandscape`
  (params (InLandscape :type "/Game/Blueprints/WorldObjects/BP_JetLandscapeMesh Object Reference"))
  (returns (bIsWithin :type Boolean))
  (bind _returnvalue (`JetLandscapeMesh.GetLandscapeScale` (`JetLandscapeMesh.LandscapeProperties` InLandscape)))
  (bind _x (.x (`self.K2_GetActorLocation` InLandscape)))
  (bind _y (.y (`self.K2_GetActorLocation` InLandscape)))
  (return (and (`KismetMathLibrary.InRange_FloatFloat` (.x (`self.K2_GetActorLocation`)) _x (+ _x _returnvalue)) (`KismetMathLibrary.InRange_FloatFloat` (.y (`self.K2_GetActorLocation`)) _y (+ _y _returnvalue)))))

(fn `UserConstructionScript`)