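; BP_JetGameState is a game state Blueprint that tracks the jet game's landscape meshes.
; Spawn and destroy events call their parent, then add or remove each BP_JetLandscapeMesh in SortedLandscapeArray.
; UpdateSortedLandscapes attempts an insertion sort by landscape-center distance to player 0's character, but returns the array unchanged.
; That sort is called only from unreachable nodes, alongside leftover debug drawing of mesh normals and distance printing.
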(event `self.ReceiveTick`
  (params (DeltaSeconds :type "Float (single-precision)")))

(event `self.OnLandscapeSpawned`
  (params (InLandscape :type "JetLandscapeMesh Object Reference") (InProcMesh :type "ProcMeshData Structure (by ref)"))
  (`parent.OnLandscapeSpawned` InLandscape InProcMesh)
  (`|ExecutionSequence`
    (:`then_0`
      (bind _asbp_jet_landscape_mesh (cast `/Game/Blueprints/WorldObjects/BP_JetLandscapeMesh` InLandscape))
      (`KismetArrayLibrary.Array_Add` (`self.SortedLandscapeArray`) _asbp_jet_landscape_mesh))
    (:`then_1`)))

(event `self.OnLandscapeDestroyed`
  (params (InLandscape :type "JetLandscapeMesh Object Reference") (InProcMesh :type "ProcMeshData Structure (by ref)"))
  (`parent.OnLandscapeDestroyed` InLandscape InProcMesh)
  (bind _asbp_jet_landscape_mesh (cast `/Game/Blueprints/WorldObjects/BP_JetLandscapeMesh` InLandscape))
  (`KismetArrayLibrary.Array_RemoveItem` (`self.SortedLandscapeArray`) _asbp_jet_landscape_mesh))

(fn `GetLandscapeLocalPlayerDistance`
  (params (BP_JetLandscape :type "/Game/Blueprints/WorldObjects/BP_JetLandscapeMesh Object Reference"))
  (returns (ReturnValue :type "Float (double-precision)"))
  (return (`KismetMathLibrary.VSize` (- (`/Game/Blueprints/WorldObjects/BP_JetLandscapeMesh.GetCenterLocation` BP_JetLandscape) (`self.K2_GetActorLocation` (`GameplayStatics.GetPlayerCharacter` 0))))))

(fn `UpdateSortedLandscapes`
  (returns (SortedLandscapeArray :type "Array of /Game/Blueprints/WorldObjects/BP_JetLandscapeMesh Object Reference"))
  (locals (LocalPlayerPosition :type "Vector Structure" :default (0.0 0.0 0.0)) (LocalSortedLandscapes :type "Array of /Game/Blueprints/WorldObjects/BP_JetLandscapeMesh Object Reference") (LocalLandscape :type "/Game/Blueprints/WorldObjects/BP_JetLandscapeMesh Object Reference") (LocalDistance :type "Float (double-precision)" :default 0.0) (NewLocalVar_0 :type "Array of Integer"))
  (set `local.LocalPlayerPosition` (`self.K2_GetActorLocation` (`GameplayStatics.GetPlayerCharacter` 0)))
  (for _array_element (`self.SortedLandscapeArray`)
    (set `local.LocalLandscape` _array_element)
    (if (> (`KismetArrayLibrary.Array_Length` (`local.LocalSortedLandscapes`)) 0)
      (for (_array_element_2 _array_index) (`local.LocalSortedLandscapes`)
        (if (< (`self.GetLandscapeLocalPlayerDistance` (`local.LocalLandscape`)) (`self.GetLandscapeLocalPlayerDistance` _array_element_2))
          (`KismetArrayLibrary.Array_Insert` (`local.LocalSortedLandscapes`) (`local.LocalLandscape`) _array_index)
          (break)))
      (else
        (`KismetArrayLibrary.Array_Add` (`local.LocalSortedLandscapes`) (`local.LocalLandscape`)))))
  (bind _output_get (set `self.SortedLandscapeArray` (`self.SortedLandscapeArray`)))
  (return _output_get))

(fn `UserConstructionScript`)