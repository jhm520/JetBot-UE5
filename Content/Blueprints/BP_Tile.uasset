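; BP_Tile is a grid tile actor that fits itself against surrounding tiles by height and rotation.
; FitTileWithNeighbors tries shuffled height steps and random-direction 90-degree turns, keeping the transform with the highest share of corner spheres hit by object traces.
; Helpers find neighbors by compass direction through tall sphere traces and map corners to directions.
; Its success flag and match count read MaxMatchingCorners, which the live path never updates.
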(fn `FindCardinalNeighborTile`
  (params (InCardinalDirection :type "/Game/Blueprints/CardinalDirection Enum" :default "NewEnumerator0"))
  (returns (OutTile :type "/Game/Blueprints/BP_Tile Object Reference"))
  (bind _returnvalue (`self.GetTileCardinalTransform` InCardinalDirection))
  (bind (_outhit _returnvalue_2) (`KismetSystemLibrary.SphereTraceSingle` (- _returnvalue (0.0 0.0 10000.0)) (+ _returnvalue (0.0 0.0 10000.0)) 30.0 "TraceTypeQuery3"))
  (if _returnvalue_2
    (bind _asbp_tile (cast `/Game/Blueprints/BP_Tile` (`.HitActor` (`GameplayStatics.BreakHitResult` _outhit))))
    (return _asbp_tile)))

(fn `FitsWithTile`
  (params (InOtherTile :type "/Game/Blueprints/BP_Tile Object Reference"))
  (returns (bDoesFit :type Boolean))
  (for _array_element (`self.GetTileCardinalCorners` (`self.GetNeighborCardinality` InOtherTile))
    (bind (_outhit _returnvalue) (`KismetSystemLibrary.SphereTraceSingleForObjects` :`Start` (- (`SceneComponent.K2_GetComponentLocation` _array_element) (0.0 0.0 5.0)) :`End` (+ (`SceneComponent.K2_GetComponentLocation` _array_element) (0.0 0.0 5.0)) :`Radius` (`SphereComponent.GetScaledSphereRadius` _array_element) :`ObjectTypes` (`|MakeArray` "ObjectTypeQuery7" :!type "EObjectTypeQuery Enum") :`DrawTime` 10.0))
    (if (not _returnvalue)
      (return false)))
  (return true))

(fn `FitTileWithNeighbors`
  (params (InHeightDiffs :type "Array of Integer"))
  (returns (bFitSuccessful :type Boolean) (MatchCount :type Integer) (MaxPercentMatch :type "Float (double-precision)"))
  (locals (LocalNeighboringTiles :type "Array of /Game/Blueprints/BP_Tile Object Reference") (bFitFound :type Boolean :default false) (RandRotBit :type Boolean) (HeightDiffs :type "Array of Integer") (MaxMatchingCorners :type Integer) (LocalMatchingCorners :type Integer :default 0) (BestTileWorldTransform :type "Transform Structure") (LocalTileFitCount :type Integer :default 0) (MaxTileFitCount :type Integer) (LocalHeightDiffs :type "Array of Integer"))
  (set `local.LocalHeightDiffs` InHeightDiffs)
  (set `local.RandRotBit` (`KismetMathLibrary.RandomBool`))
  (`|ExecutionSequence`
    (:`then_0`
      (if (> (`KismetArrayLibrary.Array_Length` (`local.LocalHeightDiffs`)) 0)
        (set `local.HeightDiffs` InHeightDiffs)))
    (:`then_1`
      (`KismetArrayLibrary.Array_Shuffle` (`local.HeightDiffs`))
      (set `self.OriginalPos` (`self.K2_GetActorLocation`))
      (for _array_element (`local.HeightDiffs`)
        (`self.K2_SetActorLocation` (+ (`self.OriginalPos`) (`KismetMathLibrary.MakeVector` 0.0 0.0 (* (* (.z (`BoxComponent.BoxExtent` (`self.Box`))) 2.0) _array_element))))
        (for _ (range 3)
          (set `local.bFitFound` true)
          (set `self.LocalPercentMatch` (`self.GetPercentMatchingTileCorners`))
          (`|ExecutionSequence`
            (:`then_0`
              (if (> (`self.LocalPercentMatch`) (`self.MaxPercentMatch`))
                (set `self.MaxPercentMatch` (`self.LocalPercentMatch`))
                (set `local.BestTileWorldTransform` (`self.GetTransform`))))
            (:`then_1`
              (`self.K2_AddActorLocalRotation` (`KismetMathLibrary.SelectRotator` (struct :`Yaw` 90.0) (struct :`Yaw` -90.0) (`local.RandRotBit`)))))))
      (`self.K2_SetActorTransform` (`local.BestTileWorldTransform`))
      (return (> (`local.MaxMatchingCorners`) 1) (`local.MaxMatchingCorners`) (`self.MaxPercentMatch`)))))

(fn `GetCornerCardinal`
  (params (InCorner :type "SphereComponent Object Reference"))
  (returns (OutCardinalDirections :type "Array of /Game/Blueprints/CardinalDirection Enum"))
  (locals (LocalOutCardinal :type "Array of /Game/Blueprints/CardinalDirection Enum"))
  (bind _x (.x (- (`SceneComponent.K2_GetComponentLocation` InCorner) (`self.K2_GetActorLocation`))))
  (bind _y (.y (- (`SceneComponent.K2_GetComponentLocation` InCorner) (`self.K2_GetActorLocation`))))
  (`|ExecutionSequence`
    (:`then_0`
      (if (and (> _x 0.0) (> _y 0.0))
        (bind _output_get (set `local.LocalOutCardinal` (`|MakeArray` "NewEnumerator0" "NewEnumerator1" "NewEnumerator2" :!type "/Game/Blueprints/CardinalDirection Enum")))
        (return _output_get)))
    (:`then_1`
      (if (and (> _x 0.0) (not (> _y 0.0)))
        (bind _output_get_2 (set `local.LocalOutCardinal` (`|MakeArray` "NewEnumerator0" "NewEnumerator7" "NewEnumerator6" :!type "/Game/Blueprints/CardinalDirection Enum")))
        (return _output_get_2)))
    (:`then_2`
      (if (and (not (> _x 0.0)) (> _y 0.0))
        (bind _output_get_3 (set `local.LocalOutCardinal` (`|MakeArray` "NewEnumerator4" "NewEnumerator3" "NewEnumerator2" :!type "/Game/Blueprints/CardinalDirection Enum")))
        (return _output_get_3)))
    (:`then_3`
      (if (and (not (> _x 0.0)) (not (> _y 0.0)))
        (bind _output_get_4 (set `local.LocalOutCardinal` (`|MakeArray` "NewEnumerator4" "NewEnumerator5" "NewEnumerator6" :!type "/Game/Blueprints/CardinalDirection Enum")))
        (return _output_get_4)))))

(fn `GetNeighborCardinality`
  (params (InNeighborTile :type "/Game/Blueprints/BP_Tile Object Reference"))
  (returns (OutCardinality :type "/Game/Blueprints/CardinalDirection Enum"))
  (bind _x (.x (- (`self.K2_GetActorLocation` InNeighborTile) (`self.K2_GetActorLocation`))))
  (bind _y (.y (- (`self.K2_GetActorLocation` InNeighborTile) (`self.K2_GetActorLocation`))))
  (`|ExecutionSequence`
    (:`then_0`
      (if (and (> _x 0.0) (== _y 0.0))
        (return "NewEnumerator0")))
    (:`then_1`
      (if (and (< _x 0.0) (== _y 0.0))
        (return "NewEnumerator4")))
    (:`then_2`
      (if (and (== _x 0.0) (> _y 0.0))
        (return "NewEnumerator2")))
    (:`then_3`
      (if (and (== _x 0.0) (< _y 0.0))
        (return "NewEnumerator6")))
    (:`then_4`
      (if (and (> _x 0.0) (> _y 0.0))
        (return "NewEnumerator1")))
    (:`then_5`
      (if (and (> _x 0.0) (not (> _y 0.0)))
        (return "NewEnumerator7")))
    (:`then_6`
      (if (and (not (> _x 0.0)) (> _y 0.0))
        (return "NewEnumerator3")))
    (:`then_7`
      (if (and (not (> _x 0.0)) (not (> _y 0.0)))
        (return "NewEnumerator5")))))

(fn `GetNeighboringTiles`
  (returns (OutNeighboringTiles :type "Array of /Game/Blueprints/BP_Tile Object Reference"))
  (locals (LocalTiles :type "Array of /Game/Blueprints/BP_Tile Object Reference"))
  (for _index (range 8)
    (bind _outtile (`self.FindCardinalNeighborTile` (cast `/Game/Blueprints/CardinalDirection` (`KismetMathLibrary.Conv_IntToByte` _index))))
    (`/Engine/EditorBlueprintResources/StandardMacros.IsValid` _outtile
      (:`Is Valid`
        (`KismetArrayLibrary.Array_AddUnique` (`local.LocalTiles`) _outtile))))
  (return (`local.LocalTiles`)))

(fn `GetNumMatchingTileCorners`
  (returns (OutMatchingCorners :type Integer))
  (locals (LocalMatchingCorners :type Integer :default 0))
  (for _array_element (`self.Corners`)
    (`/Engine/EditorBlueprintResources/StandardMacros.IsValid` _array_element
      (:`Is Valid`
        (bind (_outhits _returnvalue) (`KismetSystemLibrary.SphereTraceMultiForObjects` (- (`SceneComponent.K2_GetComponentLocation` _array_element) (0.0 0.0 10.0)) (+ (`SceneComponent.K2_GetComponentLocation` _array_element) (0.0 0.0 10.0)) (`SphereComponent.GetScaledSphereRadius` _array_element) (`|MakeArray` "ObjectTypeQuery7" :!type "EObjectTypeQuery Enum")))
        (if _returnvalue
          (`/Engine/EditorBlueprintResources/StandardMacros.IncrementInt` (`local.LocalMatchingCorners`)
            (:`  `
              (set `local.LocalMatchingCorners` (+ (`local.LocalMatchingCorners`) (`KismetArrayLibrary.Array_Length` _outhits)))))))))
  (return (`local.LocalMatchingCorners`)))

(fn `GetPercentMatchingTileCorners`
  (returns (OutPercentMatch :type "Float (double-precision)"))
  (locals (LocalMatchingCorners :type Integer :default 0))
  (for _array_element (`self.Corners`)
    (`/Engine/EditorBlueprintResources/StandardMacros.IsValid` _array_element
      (:`Is Valid`
        (bind (_outhits _returnvalue) (`KismetSystemLibrary.SphereTraceMultiForObjects` (- (`SceneComponent.K2_GetComponentLocation` _array_element) (0.0 0.0 5.0)) (+ (`SceneComponent.K2_GetComponentLocation` _array_element) (0.0 0.0 5.0)) (`SphereComponent.GetScaledSphereRadius` _array_element) (`|MakeArray` "ObjectTypeQuery7" :!type "EObjectTypeQuery Enum")))
        (if _returnvalue
          (`/Engine/EditorBlueprintResources/StandardMacros.IncrementInt` (`local.LocalMatchingCorners`))))))
  (return (/ (`KismetMathLibrary.Conv_IntToDouble` (`local.LocalMatchingCorners`)) (`KismetMathLibrary.Conv_IntToDouble` (`self.CornersNum`)))))

(fn `GetTileCardinalCorners`
  (params (InCardinalDirection :type "/Game/Blueprints/CardinalDirection Enum" :default "NewEnumerator0"))
  (returns (OutCorners :type "Array of SphereComponent Object Reference"))
  (locals (LocalOutCorners :type "Array of SphereComponent Object Reference"))
  (`|ExecutionSequence`
    (:`then_0`
      (if (`self.IsCornerCardinal` (`self.Corner`) InCardinalDirection)
        (`KismetArrayLibrary.Array_AddUnique` (`local.LocalOutCorners`) (`self.Corner`))))
    (:`then_1`
      (if (`self.IsCornerCardinal` (`self.Corner1`) InCardinalDirection)
        (`KismetArrayLibrary.Array_AddUnique` (`local.LocalOutCorners`) (`self.Corner1`))))
    (:`then_2`
      (if (`self.IsCornerCardinal` (`self.Corner2`) InCardinalDirection)
        (`KismetArrayLibrary.Array_AddUnique` (`local.LocalOutCorners`) (`self.Corner2`))))
    (:`then_3`
      (if (`self.IsCornerCardinal` (`self.Corner3`) InCardinalDirection)
        (`KismetArrayLibrary.Array_AddUnique` (`local.LocalOutCorners`) (`self.Corner3`))))
    (:`then_4`
      (return (`local.LocalOutCorners`)))))

(fn `GetTileCardinalTransform`
  (params (InCardinalDirection :type "/Game/Blueprints/CardinalDirection Enum" :default "NewEnumerator0"))
  (returns (ReturnValue :type "Vector Structure"))
  (bind _returnvalue (* (.x (`BoxComponent.BoxExtent` (`self.Box`))) -2.0))
  (bind _returnvalue_2 (* (.x (`BoxComponent.BoxExtent` (`self.Box`))) 2.0))
  (return (+ (.location (`self.GetTransform`)) (select `/Game/Blueprints/CardinalDirection` InCardinalDirection :`NewEnumerator0` (`KismetMathLibrary.MakeVector` _returnvalue_2) :`NewEnumerator1` (`KismetMathLibrary.MakeVector` _returnvalue_2 _returnvalue_2) :`NewEnumerator2` (`KismetMathLibrary.MakeVector` 0.0 _returnvalue_2) :`NewEnumerator3` (`KismetMathLibrary.MakeVector` _returnvalue _returnvalue_2) :`NewEnumerator4` (`KismetMathLibrary.MakeVector` _returnvalue) :`NewEnumerator5` (`KismetMathLibrary.MakeVector` _returnvalue _returnvalue) :`NewEnumerator6` (`KismetMathLibrary.MakeVector` 0.0 _returnvalue) :`NewEnumerator7` (`KismetMathLibrary.MakeVector` _returnvalue_2 _returnvalue)))))

(fn `GetTileMatchingCorners`
  (returns (CornerMatchNum :type Integer))
  (locals (LocalNeighboringTiles :type "Array of /Game/Blueprints/BP_Tile Object Reference") (LocalMatchingCorners :type Integer :default 0))
  (for _array_element (`self.Corners`)
    (`/Engine/EditorBlueprintResources/StandardMacros.IsValid` _array_element
      (:`Is Valid`
        (bind (_outhit _returnvalue) (`KismetSystemLibrary.SphereTraceSingleForObjects` :`Start` (- (`SceneComponent.K2_GetComponentLocation` _array_element) (0.0 0.0 20.0)) :`End` (+ (`SceneComponent.K2_GetComponentLocation` _array_element) (0.0 0.0 20.0)) :`Radius` (`SphereComponent.GetScaledSphereRadius` _array_element) :`ObjectTypes` (`|MakeArray` "ObjectTypeQuery7" :!type "EObjectTypeQuery Enum") :`DrawTime` 10.0))
        (if _returnvalue
          (`/Engine/EditorBlueprintResources/StandardMacros.IncrementInt` (`local.LocalMatchingCorners`))))))
  (return (`local.LocalMatchingCorners`)))

(fn `IsCornerCardinal`
  (params (InCorner :type "SphereComponent Object Reference") (InCardinal :type "/Game/Blueprints/CardinalDirection Enum" :default "NewEnumerator0"))
  (returns (bIsCardinal :type Boolean))
  (return (`KismetArrayLibrary.Array_Contains` (`self.GetCornerCardinal` InCorner) InCardinal)))

(fn `UserConstructionScript`
  (bind _output_get (set `self.Corners` (`|MakeArray` (`self.Corner`) (`self.Corner1`) (`self.Corner2`) (`self.Corner3`) (`self.Corner5`) (`self.Corner6`) (`self.Corner7`) (`self.Corner4`))))
  (set `self.CornersNum` (`KismetArrayLibrary.Array_Length` _output_get)))