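; World tile spawner that, when Active, procedurally grows a tile map outward from a StartingTile in eight directions.
; Tick expands one frontier tile per frame, shuffling and swapping the frontier each cycle up to MaxTileSpawnCycles.
; Each slot trial-spawns every shuffled tile class, scores its fit against neighbors, then spawns the best.
; A final congruency pass marks and attempts to refit mismatched tiles; several older experiments remain disconnected.
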(event `self.ReceiveBeginPlay`
  (`parent.ReceiveBeginPlay`)
  (if (`self.bActive`)
    (bind _startingtile (`self.StartingTile`)
      (:`then`
        (`/Engine/EditorBlueprintResources/StandardMacros.IncrementInt` (`self.TileCount`)
          (:`  `
            (`KismetArrayLibrary.Array_Add` (`self.WorldTiles`) _startingtile)
            (set `self.SpawnStructs` (`.OutSpawnStructs` (`/Game/Blueprints/BP_Tile.GetNeighborSpawnStructs` _startingtile)))
            (bind _outtiles1 (`self.SpawnNeighborTiles` _startingtile))
            (`KismetArrayLibrary.Array_Append` (`self.SpawningNeighbors`) _outtiles1)
            (`KismetArrayLibrary.Array_Shuffle` (`self.SpawningNeighbors`)))))
      (:`else`))))

(event `self.ReceiveTick`
  (params (DeltaSeconds :type "Float (single-precision)"))
  (`parent.ReceiveTick` DeltaSeconds)
  (if (< (`self.NumCycles`) (`self.MaxTileSpawnCycles`))
    (if (> (`KismetArrayLibrary.Array_Length` (`self.SpawningNeighbors`)) 0)
      (if (`KismetArrayLibrary.Array_IsValidIndex` (`self.SpawningNeighbors`) (`self.CurrentSpawningTileIndex`))
        (bind _outtiles1 (`self.SpawnNeighborTiles` (`|GetArrayItem` (`self.SpawningNeighbors`) (`self.CurrentSpawningTileIndex`))))
        (`KismetArrayLibrary.Array_Append` (`self.SwapArray`) _outtiles1)
        (`/Engine/EditorBlueprintResources/StandardMacros.IncrementInt` (`self.CurrentSpawningTileIndex`))
        (else
          (`KismetArrayLibrary.Array_Shuffle` (`self.SwapArray`))
          (set `self.SpawningNeighbors` (`self.SwapArray`))
          (`/Engine/EditorBlueprintResources/StandardMacros.IncrementInt` (`self.NumCycles`)
            (:`  `
              (set `self.CurrentSpawningTileIndex` 0)
              (`KismetArrayLibrary.Array_Clear` (`self.SwapArray`))
              (`KismetSystemLibrary.PrintString` (`KismetStringLibrary.Conv_IntToString` (`KismetArrayLibrary.Array_Length` (`self.WorldTiles`))) true true (struct :`G` 0.66 :`B` 1.0 :`A` 1.0) 10.0))))))
    (else
      (`/Engine/EditorBlueprintResources/StandardMacros.DoOnce` false
        (:`Completed`
          (`KismetSystemLibrary.PrintString` "World Spawn Completed!" true true (struct :`G` 0.66 :`B` 1.0 :`A` 1.0) 25.0)
          (`self.VerifyCongruency`))))))

(event `VerifyCongruency`
  (`KismetArrayLibrary.Array_Shuffle` (`self.WorldTiles`))
  (for _array_element (`self.WorldTiles`)
    (`/Engine/EditorBlueprintResources/StandardMacros.IsValid` _array_element
      (:`Is Valid`
        (if (< (`/Game/Blueprints/BP_Tile.GetPercentCongruency` _array_element) 1.0)
          (`KismetSystemLibrary.DrawDebugSphere` (`self.K2_GetActorLocation` _array_element) 300.0 12 (struct :`R` 1.0 :`B` 0.027472 :`A` 1.0) 2.0 1.0)
          (bind _outtile (`self.RefitSpawn` _array_element))
          (`KismetSystemLibrary.PrintString` (`KismetStringLibrary.Conv_DoubleToString` (`/Game/Blueprints/BP_Tile.GetPercentCongruency` _outtile)) true true (struct :`G` 0.66 :`B` 1.0 :`A` 1.0) 10.0))))))

(fn `GetBestTileSpawn`
  (params (TileTransform :type "Transform Structure") (InCurrentTIle :type "/Game/Blueprints/BP_Tile Object Reference"))
  (returns (BestTileClass1 :type "/Game/Blueprints/BP_Tile Class Reference") (BestTileTransform1 :type "Transform Structure") (MaxPercentMatch1 :type "Float (double-precision)"))
  (locals (LocalHeightDiffs :type "Array of Integer") (LocalMatchingCorners :type Integer) (LocalPercentMatch :type "Float (double-precision)") (MaxPercentMatch :type "Float (double-precision)") (BestTileClass :type "/Game/Blueprints/BP_Tile Class Reference") (BestTileTransform :type "Transform Structure") (LocalTileClasses :type "Array of /Game/Blueprints/BP_Tile Class Reference") (LocalOGCongruency :type "Float (double-precision)" :default 0.0))
  (set `local.LocalTileClasses` (`self.WorldTileClasses`))
  (set `local.LocalOGCongruency` (`/Game/Blueprints/BP_Tile.GetPercentCongruency` InCurrentTIle))
  (`KismetArrayLibrary.Array_Shuffle` (`local.LocalTileClasses`))
  (for _array_element (`local.LocalTileClasses`)
    (set `local.LocalPercentMatch` 0.0)
    (bind _returnvalue (`|SpawnActorFromClass` _array_element TileTransform "AlwaysSpawn" "OverrideRootScale" null null))
    (bind (_bfitsuccessful _matchcount _maxpercentmatch _besttileworldtransform1) (`/Game/Blueprints/BP_Tile.FitTileWithNeighbors` _returnvalue (`local.LocalHeightDiffs`)))
    (set `local.LocalMatchingCorners` _matchcount)
    (set `local.LocalPercentMatch` _maxpercentmatch)
    (`|ExecutionSequence`
      (:`then_0`
        (if (and (> (`local.LocalPercentMatch`) (`local.MaxPercentMatch`)) (> (`local.LocalPercentMatch`) (`local.LocalOGCongruency`)))
          (set `local.MaxPercentMatch` (`local.LocalPercentMatch`))
          (set `local.BestTileClass` _array_element)
          (set `local.BestTileTransform` _besttileworldtransform1)))
      (:`then_1`
        (`self.K2_DestroyActor` _returnvalue))))
  (return (`local.BestTileClass`) (`local.BestTileTransform`) (`local.MaxPercentMatch`)))

(fn `RefitSpawn`
  (params (InTile :type "/Game/Blueprints/BP_Tile Object Reference"))
  (returns (OutTile :type "/Game/Blueprints/BP_Tile Object Reference"))
  (locals (LocalOriginalFitPercent :type "Float (double-precision)" :default 0.0) (LocalTileClasses :type "Array of /Game/Blueprints/BP_Tile Class Reference") (LocalOGClass :type "/Game/Blueprints/BP_Tile Class Reference") (LocalOGTransform :type "Transform Structure") (LocalOGTIle :type "/Game/Blueprints/BP_Tile Object Reference") (LocalIndex :type Integer :default 0))
  (bind _worldtiles (`self.WorldTiles`))
  (`/Engine/EditorBlueprintResources/StandardMacros.IsValid` InTile
    (:`Is Valid`
      (set `local.LocalOGTIle` InTile)
      (set `local.LocalOriginalFitPercent` (`/Game/Blueprints/BP_Tile.GetPercentCongruency` InTile))
      (set `local.LocalOGClass` (`GameplayStatics.GetObjectClass` InTile))
      (bind _output_get (set `local.LocalOGTransform` (`self.GetTransform` InTile)))
      (bind (_besttileclass1 _besttiletransform1 _maxpercentmatch1) (`self.GetBestTileSpawn` _output_get InTile))
      (if (or (not (== (`local.LocalOGTransform`) _besttiletransform1)) (not (== _besttileclass1 (`local.LocalOGClass`))) (> _maxpercentmatch1 (`local.LocalOriginalFitPercent`)))
        (`KismetSystemLibrary.PrintString` "Tile Refit!" true true (struct :`G` 0.66 :`B` 1.0 :`A` 1.0) 5.0)
        (set `local.LocalIndex` (`KismetArrayLibrary.Array_Find` (`self.WorldTiles`) (`local.LocalOGTIle`)))
        (bind _returnvalue (`|SpawnActorFromClass` _besttileclass1 _besttiletransform1 "AlwaysSpawn" "OverrideRootScale" null null))
        (`/Engine/EditorBlueprintResources/StandardMacros.IsValid` _returnvalue
          (:`Is Valid`
            (`self.K2_DestroyActor` (`|GetArrayItem` _worldtiles (`local.LocalIndex`)))
            (`KismetArrayLibrary.Array_Insert` _worldtiles _returnvalue (`local.LocalIndex`))
            (return _returnvalue)))
        (else
          (`KismetSystemLibrary.PrintString` "Perfect Fit!" true true (struct :`G` 0.66 :`B` 1.0 :`A` 1.0) 5.0))))))

(fn `SpawnAttachedTile`
  (params (InputTile :type "/Game/Blueprints/BP_Tile Object Reference") (InTilePosition :type "/Game/Blueprints/CardinalDirection Enum" :default "NewEnumerator0"))
  (returns (NewTile :type "/Game/Blueprints/BP_Tile Object Reference"))
  (locals (LocalTileClasses :type "Array of /Game/Blueprints/BP_Tile Class Reference") (bTileSpawnValid :type Boolean) (MaxMatchingCorners :type Integer :default 0) (LoopCount :type Integer) (CurrentTileClassIdx :type Integer) (NewLocalVar_0 :type Integer :default 0) (LocalMatchingCorners :type Integer :default 0) (BestTileClass :type "/Game/Blueprints/BP_Tile Class Reference") (BestTileTransform :type "Transform Structure") (LocalHeightDiffs :type "Array of Integer") (LocalRampUpHeightDiffs :type "Array of Integer") (LocalPercentMatch :type "Float (double-precision)" :default 0.0) (MaxPercentMatch :type "Float (double-precision)" :default -1.0))
  (bind _worldtileclasses (`self.WorldTileClasses`))
  (bind _localheightdiffs (`local.LocalHeightDiffs`))
  (`/Engine/EditorBlueprintResources/StandardMacros.IsValid` InputTile
    (:`Is Valid`
      (`/Engine/EditorBlueprintResources/StandardMacros.IsValid` (`/Game/Blueprints/BP_Tile.FindCardinalNeighborTile` InputTile InTilePosition)
        (:`Is Valid`
          (return null) ; If there was already a tile spawned here, don't spawn another one
        )
        (:`Is Not Valid`
          (set `self.bRampUp` (`KismetMathLibrary.RandomBool`))
          (set `local.LocalTileClasses` (select `bool` (`self.bRampUp`) :`false` _worldtileclasses :`true` _worldtileclasses))
          (`KismetArrayLibrary.Array_Shuffle` (`local.LocalTileClasses`))
          (set `local.CurrentTileClassIdx` 0)
          (for _array_element (`local.LocalTileClasses`)
            (set `local.bTileSpawnValid` false)
            (bind _returnvalue (`|SpawnActorFromClass` _array_element (`KismetMathLibrary.MakeTransform` (`/Game/Blueprints/BP_Tile.GetTileCardinalTransform` InputTile InTilePosition)) "AlwaysSpawn" "OverrideRootScale" null null))
            (bind (_bfitsuccessful _matchcount _maxpercentmatch) (`/Game/Blueprints/BP_Tile.FitTileWithNeighbors` _returnvalue (select `bool` (`self.bRampUp`) :`false` _localheightdiffs :`true` _localheightdiffs)))
            (set `local.LocalMatchingCorners` _matchcount)
            (set `local.LocalPercentMatch` _maxpercentmatch)
            (`|ExecutionSequence`
              (:`then_0`
                (if (> (`local.LocalPercentMatch`) (`local.MaxPercentMatch`))
                  (set `local.MaxPercentMatch` (`local.LocalPercentMatch`))
                  (set `local.BestTileClass` _array_element)
                  (set `local.BestTileTransform` (`self.GetTransform` _returnvalue))))
              (:`then_1`
                (`self.K2_DestroyActor` _returnvalue))))
          (bind _returnvalue_2 (`|SpawnActorFromClass` (`local.BestTileClass`) (`local.BestTileTransform`) "AlwaysSpawn" "OverrideRootScale" null null))
          (`|ExecutionSequence`
            (:`then_0`
              (`/Engine/EditorBlueprintResources/StandardMacros.IsValid` _returnvalue_2
                (:`Is Valid`
                  (`KismetArrayLibrary.Array_Add` (`self.WorldTiles`) _returnvalue_2)
                  (`/Engine/EditorBlueprintResources/StandardMacros.IncrementInt` (`self.TileCount`)))))
            (:`then_1`
              (return _returnvalue_2))))))))

(fn `SpawnNeighborTiles`
  (params (InTile :type "/Game/Blueprints/BP_Tile Object Reference"))
  (returns (OutTiles1 :type "Array of /Game/Blueprints/BP_Tile Object Reference"))
  (locals (OutTiles :type "Array of /Game/Blueprints/BP_Tile Object Reference"))
  (for _index (range 8)
    (bind _newtile (`self.SpawnAttachedTile` InTile (cast `/Game/Blueprints/CardinalDirection` (`KismetMathLibrary.Conv_IntToByte` _index))))
    (`/Engine/EditorBlueprintResources/StandardMacros.IsValid` _newtile
      (:`Is Valid`
        (`KismetArrayLibrary.Array_AddUnique` (`local.OutTiles`) _newtile))))
  (return (`local.OutTiles`)))

(fn `SpawnTile`
  (params (InSpawnStruct :type "/Game/Blueprints/WorldTiles/WorldTileSpawnStruct Structure"))
  (returns (NewTile :type "/Game/Blueprints/BP_Tile Object Reference"))
  (locals (LocalHeightDiffs :type "Array of Integer") (LocalMatchingCorners :type Integer) (LocalPercentMatch :type "Float (double-precision)") (MaxPercentMatch :type "Float (double-precision)") (BestTileClass :type "/Game/Blueprints/BP_Tile Class Reference") (BestTileTransform :type "Transform Structure") (LocalTileClasses :type "Array of /Game/Blueprints/BP_Tile Class Reference"))
  (bind (_spawntransform _cardinaldirection _attachedtile) (break `/Game/Blueprints/WorldTiles/WorldTileSpawnStruct` InSpawnStruct))
  (`/Engine/EditorBlueprintResources/StandardMacros.IsValid` (`/Game/Blueprints/BP_Tile.FindCardinalNeighborTile` _attachedtile _cardinaldirection)
    (:`Is Valid`
      (return null) ; If there was already a tile spawned here, don't spawn another one
    )
    (:`Is Not Valid`
      (set `local.LocalTileClasses` (`self.WorldTileClasses`))
      (`KismetArrayLibrary.Array_Shuffle` (`local.LocalTileClasses`))
      (for _array_element (`local.LocalTileClasses`)
        (bind _returnvalue (`|SpawnActorFromClass` _array_element (`.SpawnTransform_2_7CD11975476BCD4FD40825A60D29FD29` (break `/Game/Blueprints/WorldTiles/WorldTileSpawnStruct` InSpawnStruct)) "AlwaysSpawn" "OverrideRootScale" null null))
        (bind (_bfitsuccessful _matchcount _maxpercentmatch) (`/Game/Blueprints/BP_Tile.FitTileWithNeighbors` _returnvalue (`local.LocalHeightDiffs`)))
        (set `local.LocalMatchingCorners` _matchcount)
        (set `local.LocalPercentMatch` _maxpercentmatch)
        (`|ExecutionSequence`
          (:`then_0`
            (if (> (`local.LocalPercentMatch`) (`local.MaxPercentMatch`))
              (set `local.MaxPercentMatch` (`local.LocalPercentMatch`))
              (set `local.BestTileClass` _array_element)
              (set `local.BestTileTransform` (`self.GetTransform` _returnvalue))))
          (:`then_1`
            (`self.K2_DestroyActor` _returnvalue))))
      (bind _returnvalue_2 (`|SpawnActorFromClass` (`local.BestTileClass`) (`local.BestTileTransform`) "AlwaysSpawn" "OverrideRootScale" null null))
      (`|ExecutionSequence`
        (:`then_1`
          (return _returnvalue_2))))))

(fn `UserConstructionScript`)