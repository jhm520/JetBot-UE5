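; World spawner that procedurally grows a tile-based world outward from a starting tile.
; Tick expands one frontier tile per frame, then shuffles and swaps in the new ring until the cycle limit is reached.
; Each expansion fills empty spots among the eight surrounding directions.
; For each spot it trial-spawns every shuffled tile class, scores it with FitTileWithNeighbors, destroys it, and respawns the best match at its fitted transform.
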(event `self.ReceiveBeginPlay`
  (`parent.ReceiveBeginPlay`)
  (bind _startingtile (`self.StartingTile`)
    (:`then`
      (`/Engine/EditorBlueprintResources/StandardMacros.IncrementInt` (`self.TileCount`)
        (:`  `
          (`KismetArrayLibrary.Array_Add` (`self.WorldTiles`) _startingtile)
          (bind _outtiles1 (`self.SpawnNeighborTiles` _startingtile))
          (`KismetArrayLibrary.Array_Append` (`self.SpawningNeighbors`) _outtiles1)
          (`KismetArrayLibrary.Array_Shuffle` (`self.SpawningNeighbors`)))))
    (:`else`)))

(event `self.ReceiveTick`
  (params (DeltaSeconds :type "Float (single-precision)"))
  (`parent.ReceiveTick` DeltaSeconds)
  (if (< (`self.NumCycles`) (`self.MaxTileSpawnCycles`))
    (if (> (`KismetArrayLibrary.Array_Length` (`self.SpawningNeighbors`)) 0)
      (if (`KismetArrayLibrary.Array_IsValidIndex` (`self.SpawningNeighbors`) (`self.CurrentSpawningTileIndex`))
        (bind _outtiles1 (`self.SpawnNeighborTiles` (`|GetArrayItem` (`self.SpawningNeighbors`) (`self.CurrentSpawningTileIndex`))))
        (`KismetArrayLibrary.Array_Append` (`self.SwapArray`) _outtiles1)
        (`/Engine/EditorBlueprintResources/StandardMacros.IncrementInt` (`self.CurrentSpawningTileIndex`))
        (else
          (`KismetArrayLibrary.Array_Shuffle` (`self.SwapArray`))
          (set `self.SpawningNeighbors` (`self.SwapArray`))
          (`/Engine/EditorBlueprintResources/StandardMacros.IncrementInt` (`self.NumCycles`)
            (:`  `
              (set `self.CurrentSpawningTileIndex` 0)
              (`KismetArrayLibrary.Array_Clear` (`self.SwapArray`))
              (`KismetSystemLibrary.PrintString` (`KismetStringLibrary.Conv_IntToString` (`KismetArrayLibrary.Array_Length` (`self.WorldTiles`))) true true (struct :`G` 0.66 :`B` 1.0 :`A` 1.0) 10.0))))))
    (else
      (`/Engine/EditorBlueprintResources/StandardMacros.DoOnce` false
        (:`Completed`
          (`KismetSystemLibrary.PrintString` "World Spawn Completed!" true true (struct :`G` 0.66 :`B` 1.0 :`A` 1.0) 25.0))))))

(fn `SpawnAttachedTile`
  (params (InputTile :type "/Game/Blueprints/BP_Tile Object Reference") (InTilePosition :type "/Game/Blueprints/CardinalDirection Enum" :default "NewEnumerator0"))
  (returns (NewTile :type "/Game/Blueprints/BP_Tile Object Reference"))
  (locals (LocalTileClasses :type "Array of /Game/Blueprints/BP_Tile Class Reference") (bTileSpawnValid :type Boolean) (MaxMatchingCorners :type Integer :default 0) (LoopCount :type Integer) (CurrentTileClassIdx :type Integer) (NewLocalVar_0 :type Integer :default 0) (LocalMatchingCorners :type Integer :default 0) (BestTileClass :type "/Game/Blueprints/BP_Tile Class Reference") (BestTileTransform :type "Transform Structure") (LocalHeightDiffs :type "Array of Integer") (LocalRampUpHeightDiffs :type "Array of Integer") (LocalPercentMatch :type "Float (double-precision)" :default 0.0) (MaxPercentMatch :type "Float (double-precision)" :default 0.0))
  (bind _worldtileclasses (`self.WorldTileClasses`))
  (bind _localheightdiffs (`local.LocalHeightDiffs`))
  (`/Engine/EditorBlueprintResources/StandardMacros.IsValid` InputTile
    (:`Is Valid`
      (`/Engine/EditorBlueprintResources/StandardMacros.IsValid` (`/Game/Blueprints/BP_Tile.FindCardinalNeighborTile` InputTile InTilePosition)
        (:`Is Valid`
          (return null) ; If there was already a tile spawned here, don't spawn another one
        )
        (:`Is Not Valid`
          (set `self.bRampUp` (`KismetMathLibrary.RandomBool`))
          (set `local.LocalTileClasses` (select `bool` (`self.bRampUp`) :`false` _worldtileclasses :`true` _worldtileclasses))
          (`KismetArrayLibrary.Array_Shuffle` (`local.LocalTileClasses`))
          (set `local.CurrentTileClassIdx` 0)
          (for _array_element (`local.LocalTileClasses`)
            (set `local.bTileSpawnValid` false)
            (bind _returnvalue (`|SpawnActorFromClass` _array_element (`KismetMathLibrary.MakeTransform` (`/Game/Blueprints/BP_Tile.GetTileCardinalTransform` InputTile InTilePosition)) "AlwaysSpawn" "OverrideRootScale" null null))
            (bind (_bfitsuccessful _matchcount _maxpercentmatch) (`/Game/Blueprints/BP_Tile.FitTileWithNeighbors` _returnvalue (select `bool` (`self.bRampUp`) :`false` _localheightdiffs :`true` _localheightdiffs)))
            (set `local.LocalMatchingCorners` _matchcount)
            (set `local.LocalPercentMatch` _maxpercentmatch)
            (`|ExecutionSequence`
              (:`then_0`
                (if (> (`local.LocalPercentMatch`) (`local.MaxPercentMatch`))
                  (set `local.MaxPercentMatch` (`local.LocalPercentMatch`))
                  (set `local.BestTileClass` _array_element)
                  (set `local.BestTileTransform` (`self.GetTransform` _returnvalue))))
              (:`then_1`
                (`self.K2_DestroyActor` _returnvalue))))
          (bind _returnvalue_2 (`|SpawnActorFromClass` (`local.BestTileClass`) (`local.BestTileTransform`) "AlwaysSpawn" "OverrideRootScale" null null))
          (`|ExecutionSequence`
            (:`then_0`
              (`/Engine/EditorBlueprintResources/StandardMacros.IsValid` _returnvalue_2
                (:`Is Valid`
                  (`KismetArrayLibrary.Array_Add` (`self.WorldTiles`) _returnvalue_2)
                  (`/Engine/EditorBlueprintResources/StandardMacros.IncrementInt` (`self.TileCount`)))))
            (:`then_1`
              (return _returnvalue_2))))))))

(fn `SpawnNeighborTiles`
  (params (InTile :type "/Game/Blueprints/BP_Tile Object Reference"))
  (returns (OutTiles1 :type "Array of /Game/Blueprints/BP_Tile Object Reference"))
  (locals (OutTiles :type "Array of /Game/Blueprints/BP_Tile Object Reference"))
  (for _index (range 8)
    (bind _newtile (`self.SpawnAttachedTile` InTile (cast `/Game/Blueprints/CardinalDirection` (`KismetMathLibrary.Conv_IntToByte` _index))))
    (`/Engine/EditorBlueprintResources/StandardMacros.IsValid` _newtile
      (:`Is Valid`
        (`KismetArrayLibrary.Array_AddUnique` (`local.OutTiles`) _newtile))))
  (return (`local.OutTiles`)))

(fn `UserConstructionScript`)